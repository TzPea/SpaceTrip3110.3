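; BP_WatermelonEnemy is a watermelon enemy that chases the player, repeatedly reissuing AI MoveTo while a timeline animates the melon's height.
; It registers in the player's EnemyArray and, on first touch, calls the player's GotShot and dies with an explosion sound.
; HitTarget lowers health and swaps damage meshes, while grenade hits and Damager kill outright.
; Death triggers Niagara, disables collision, then gates an ammo drop and destruction behind a random MultiGate.
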(event OnComponentHit(Melon)
  (params (HitComponent :type Primitive%20Component%20Object%20Reference) (OtherActor :type Actor%20Object%20Reference) (OtherComp :type Primitive%20Component%20Object%20Reference) (NormalImpulse :type Vector :default "0, 0, 0") (Hit :type Hit%20Result%20Structure%20%28by%20ref%29))
  ;[1 0 1 1 100] Grenade Hit Death
  (bind _asbp_melon_grenade (Utilities|Casting|CastToBP_MelonGrenade OtherActor))
  (Default|Explode _asbp_melon_grenade)
  (CallFunction|DiebyGrenadeHit))

(event OnComponentBeginOverlap(Melon)
  (params (OverlappedComponent :type Primitive%20Component%20Object%20Reference) (OtherActor :type Actor%20Object%20Reference) (OtherComp :type Primitive%20Component%20Object%20Reference) (OtherBodyIndex :type Integer) (bFromSweep :type Boolean) (SweepResult :type Hit%20Result%20Structure%20%28by%20ref%29))
  (bind _asbp_first_person_character (Utilities|Casting|CastToBP_FirstPersonCharacter OtherActor))
  (Utilities|FlowControl|DoOnce false
    (:Completed
      (Audio|PlaySoundatLocation "/Game/StarterContent/Audio/Explosion01.Explosion01" "0, 0, 0" "0, 0, 0" 1.0 1.0 0.0 0 0 0 0)
      (Default|GotShot _asbp_first_person_character)
      (CallFunction|Death))))

(event Custom|DieByGrenadeHit
  (bind _melon (Variables|Default|GetMelon))
  (CallFunction|Death)
  (Rendering|Material|SetMaterial _melon 0 "/Game/MyStuff/MyMaterials/MAT_DeadMelon.MAT_DeadMelon")
  (Components|StaticMesh|SetStaticMesh _melon "/Game/MyStuff/MyMeshes/MelonDead.MelonDead")
  (Utilities|FlowControl|Delay 3.0)
  (Components|StaticMesh|SetStaticMesh _melon 0))

(event Custom|GoToPlayer
  (Variables|/Script/Engine.CharacterMovementComponent|SetMaxWalkSpeed (Variables|Character|GetCharacterMovement) (Variables|Default|GetMax%20Walk%20Speed))
  (AI|AIMoveTo self "0, 0, 0" (Game|GetPlayerCharacter 0) 1e+01 false
    (:OnSuccess
      _)
    (:OnFail
      _))
  (Utilities|FlowControl|Delay 2.0)
  (CallFunction|GotoPlayer))

(event Custom|Death
  (Components|Activation|Activate (Variables|Default|GetNiagara) false)
  (Collision|SetCollisionEnabled (Variables|Collision|GetCapsuleComponent) "NoCollision")
  (Utilities|FlowControl|Delay 4.0)
  ;[1 0 1 1 100] DropAmmo
  (Utilities|FlowControl|MultiGate true true -1
    (:Out%200
      (Game|SpawnActorfromClass "/Game/MyStuff/MyBlueprints/BP_MelonAmmoPickUp.BP_MelonAmmoPickUp_C" (Math|Transform|MakeTransform (Transformation|GetWorldLocation (Variables|Collision|GetCapsuleComponent)) "0, 0, 0" "1.000000,1.000000,1.000000") "Undefined" "OverrideRootScale" 0 0)
      (Actor|DestroyActor))))

(event Custom|HitTarget
  (bind _melon (Variables|Default|GetMelon))
  (bind _result (Math|Integer|DecrementInt (Variables|Default|GetHealth))
    (:%20%20
      (bind _output_get (Variables|Default|SetHealth _result))
      (switch int _output_get
        (:0
          (CallFunction|Death)
          (Rendering|Material|SetMaterial _melon 0 "/Game/MyStuff/MyMaterials/MAT_DeadMelon.MAT_DeadMelon")
          (Components|StaticMesh|SetStaticMesh _melon "/Game/MyStuff/MyMeshes/MelonDead.MelonDead")
          (Utilities|FlowControl|Delay 3.0)
          (Components|StaticMesh|SetStaticMesh _melon 0))
        (:3
          (Rendering|Material|SetMaterial _melon 0 "/Game/MyStuff/MyMaterials/MAT_MelonLowHealth.MAT_MelonLowHealth")
          (Components|StaticMesh|SetStaticMesh _melon "/Game/MyStuff/MyMeshes/MelonLow.MelonLow"))
        (:6
          (Rendering|Material|SetMaterial _melon 0 "/Game/MyStuff/MyMaterials/MAT_MelonMidHealth.MAT_MelonMidHealth")
          (Components|StaticMesh|SetStaticMesh _melon "/Game/MyStuff/MyMeshes/MelonMid.MelonMid"))))))

(event EventBeginPlay
  (bind _asbp_first_person_character (Utilities|Casting|CastToBP_FirstPersonCharacter (Game|GetPlayerCharacter 0)))
  (Variables|Default|SetPlayer _asbp_first_person_character)
  (Utilities|Array|Add (Variables|/Game/FPS_Stuff/FirstPerson/Blueprints/BP_FirstPersonCharacter.BP_FirstPersonCharacter_C|GetEnemyArray _asbp_first_person_character) self)
  (CallFunction|GotoPlayer)
  (bind _zaxis (Timeline|Timeline Play)
    (:Update
      (Transformation|SetRelativeLocation (Variables|Default|GetMelon) (Math|Vector|MakeVector 0.0 0.0 _zaxis) false false))))

(event EventDamager
  ;[1 0 1 1 100] HitByAoe
  (CallFunction|Death))

(fn ConstructionScript)