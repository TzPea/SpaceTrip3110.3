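; BP_PineappleTank is an enemy character that chases the player and lobs grenades at them.
; It re-issues AI MoveTo after a delay, bobs its Melon mesh on a timeline, and fires from Tick through a delay-reset DoOnce.
; Melon grenade hits and AoE damage decrement health, recoloring the mesh at thresholds.
; Death triggers Niagara, randomly drops melon ammo, and decrements the player's enemy count before destroying itself.
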(event OnComponentHit(Melon)
  (params (HitComponent :type Primitive%20Component%20Object%20Reference) (OtherActor :type Actor%20Object%20Reference) (OtherComp :type Primitive%20Component%20Object%20Reference) (NormalImpulse :type Vector :default "0, 0, 0") (Hit :type Hit%20Result%20Structure%20%28by%20ref%29))
  ;[1 0 1 1 100] Grenade Hit Death
  (bind _asbp_melon_grenade (Utilities|Casting|CastToBP_MelonGrenade OtherActor))
  (Default|Explode _asbp_melon_grenade)
  (CallFunction|HitTarget))

(event Custom|GoToPlayer
  ;[1 0 1 1 100] GoToPlayer
  (Variables|/Script/Engine.CharacterMovementComponent|SetMaxWalkSpeed (Variables|Character|GetCharacterMovement) (Variables|Default|GetMax%20Walk%20Speed))
  (AI|AIMoveTo self "0, 0, 0" (Game|GetPlayerCharacter 0) 1e+01 false
    (:OnSuccess
      _)
    (:OnFail
      _))
  (Utilities|FlowControl|Delay 2.0)
  (CallFunction|GotoPlayer))

(event Custom|Death
  (Components|Activation|Activate (Variables|Default|GetNiagara) false)
  (Collision|SetCollisionEnabled (Variables|Collision|GetCapsuleComponent) "NoCollision")
  (Utilities|FlowControl|Delay 4.0)
  (Utilities|FlowControl|MultiGate true true -1
    (:Out%200
      (Game|SpawnActorfromClass "/Game/MyStuff/MyBlueprints/BP_MelonAmmoPickUp.BP_MelonAmmoPickUp_C" (Math|Transform|MakeTransform (Transformation|GetWorldLocation (Variables|Collision|GetCapsuleComponent)) "0, 0, 0" "1.000000,1.000000,1.000000") "Undefined" "OverrideRootScale" 0 0))
    (:Out%201
      _))
  (Default|DecrementEnemies (Variables|Default|GetPlayer))
  (Actor|DestroyActor))

(event Custom|HitTarget
  (bind _melon (Variables|Default|GetMelon))
  (bind _result (Math|Integer|DecrementInt (Variables|Default|GetHealth))
    (:%20%20
      (bind _output_get (Variables|Default|SetHealth _result))
      (if (<= _output_get 0)
        (CallFunction|Death)
        (Rendering|Material|SetMaterial _melon 0 "/Game/Materials/M-ReddishPurple.M-ReddishPurple")
        (Utilities|FlowControl|Delay 3.0)
        (elif (<= _output_get 20)
          (Rendering|Material|SetMaterial _melon 0 "/Game/MyStuff/MyMaterials/MI_Red.MI_Red")
          (elif (<= _output_get 50)
            (Rendering|Material|SetMaterial _melon 0 "/Game/MyStuff/MyMaterials/MI_Yellow.MI_Yellow")))))))

(event Custom|TankFire
  (bind _returnvalue (Game|GetPlayerCharacter 0))
  (bind _spawngrenade (Variables|Default|GetSpawnGrenade))
  (bind _returnvalue_2 (Transformation|GetWorldLocation _spawngrenade))
  (bind _capsulecomponent (Variables|/Script/Engine.Character|GetCapsuleComponent _returnvalue))
  (bind _returnvalue_3 (Transformation|GetWorldLocation _capsulecomponent))
  ;[1 0 1 1 100] Firing Logic
  (Utilities|FlowControl|DoOnce false) ; enters at Reset
)

(event EventBeginPlay
  (bind _asbp_first_person_character (Utilities|Casting|CastToBP_FirstPersonCharacter (Game|GetPlayerCharacter 0)))
  (Variables|Default|SetPlayer _asbp_first_person_character)
  (Utilities|Array|Add (Variables|/Game/FPS_Stuff/FirstPerson/Blueprints/BP_FirstPersonCharacter.BP_FirstPersonCharacter_C|GetEnemyArray _asbp_first_person_character) self)
  (CallFunction|GotoPlayer)
  (bind _zaxis (Timeline|Timeline Play)
    (:Update
      (Transformation|SetRelativeLocation (Variables|Default|GetMelon) (Math|Vector|MakeVector 0.0 0.0 _zaxis) false false))))

(event EventTick
  (params (DeltaSeconds :type Float%20%28single-precision%29))
  (bind _returnvalue (Game|GetPlayerCharacter 0))
  (bind _spawngrenade (Variables|Default|GetSpawnGrenade))
  (bind _returnvalue_2 (Transformation|GetWorldLocation _spawngrenade))
  (bind _capsulecomponent (Variables|/Script/Engine.Character|GetCapsuleComponent _returnvalue))
  (bind _returnvalue_3 (Transformation|GetWorldLocation _capsulecomponent))
  ;[1 0 1 1 100] Firing Logic
  (Utilities|FlowControl|DoOnce false
    (:Completed
      (bind _returnvalue_4 (Game|SpawnActorfromClass "/Game/MyStuff/MyBlueprints/BP_EnemyGrenade.BP_EnemyGrenade_C" (Math|Transform|MakeTransform _returnvalue_2 (Math|Rotator|FindLookatRotation _returnvalue_2 _returnvalue_3) "1.000000,1.000000,1.000000") "Undefined" "MultiplyWithRoot" 0 "0.000000,0.000000,0.000000" 0))
      (Default|Launch _returnvalue_4 _returnvalue_2 _returnvalue_3)
      (Utilities|FlowControl|Delay 2.0)
      (CallFunction|TankFire))))

(event EventDamager
  ;[1 0 1 1 100] HitByAoe
  (CallFunction|HitTarget))

(fn ConstructionScript)