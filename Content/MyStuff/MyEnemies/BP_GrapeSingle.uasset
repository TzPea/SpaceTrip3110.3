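; BP_GrapeSingle is a grape enemy that chases the player with a repeating AIMoveTo, retrying a second after each success or failure.
; A timeline moves its HitBox vertically, and overlapping the player calls GotShot on them once, then kills the grape.
; A melon grenade hit explodes the grenade and kills it, while Damager hits reduce Health, swapping to a low-health material before death.
; Death hides the mesh, activates Niagara, disables collision and destroys the actor after a delay.
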(event OnComponentBeginOverlap(HitBox)
  (params (OverlappedComponent :type Primitive%20Component%20Object%20Reference) (OtherActor :type Actor%20Object%20Reference) (OtherComp :type Primitive%20Component%20Object%20Reference) (OtherBodyIndex :type Integer) (bFromSweep :type Boolean) (SweepResult :type Hit%20Result%20Structure%20%28by%20ref%29))
  (bind _asbp_first_person_character (Utilities|Casting|CastToBP_FirstPersonCharacter OtherActor))
  (Utilities|FlowControl|DoOnce false
    (:Completed
      (Default|GotShot _asbp_first_person_character)
      (CallFunction|Death))))

(event OnComponentHit(HitBox)
  (params (HitComponent :type Primitive%20Component%20Object%20Reference) (OtherActor :type Actor%20Object%20Reference) (OtherComp :type Primitive%20Component%20Object%20Reference) (NormalImpulse :type Vector :default "0, 0, 0") (Hit :type Hit%20Result%20Structure%20%28by%20ref%29))
  ;[1 0 1 1 100] Grenade Hit Death
  (bind _asbp_melon_grenade (Utilities|Casting|CastToBP_MelonGrenade OtherActor))
  (Default|Explode _asbp_melon_grenade)
  (CallFunction|Death))

(event Custom|Death
  ;[1 0 1 1 100] Death Logic
  (Rendering|SetVisibility (Variables|Default|GetSphere2) false false)
  (Components|Activation|Activate (Variables|Default|GetNiagara) false)
  (Collision|SetCollisionEnabled (Variables|Collision|GetCapsuleComponent) "NoCollision")
  (Utilities|FlowControl|Delay 1.0)
  (Actor|DestroyActor))

(event Custom|GoToPlayer
  ;[1 0 1 1 100] Chase Player
  (Variables|/Script/Engine.CharacterMovementComponent|SetMaxWalkSpeed (Variables|Character|GetCharacterMovement) (Variables|Default|GetMax%20Walk%20Speed))
  (AI|AIMoveTo self "0, 0, 0" (Game|GetPlayerCharacter 0) 0.0 false
    (:OnSuccess
      _)
    (:OnFail
      _))
  (Utilities|FlowControl|Delay 1.0)
  (CallFunction|GotoPlayer))

(event Custom|HitTarget
  ;[1 0 1 1 100] Getting Hit
  (bind _result (Math|Integer|DecrementInt (Variables|Default|GetHealth))
    (:%20%20
      (bind _output_get (Variables|Default|SetHealth _result))
      (switch int _output_get
        (:0
          (CallFunction|Death))
        (:1
          (Rendering|Material|SetMaterial (Variables|Default|GetSphere2) 0 "/Game/MyStuff/MyMaterials/MAT_GrapeLowHealth.MAT_GrapeLowHealth"))))))

(event EventBeginPlay
  ;[1 0 1 1 100] Movement
  (CallFunction|GotoPlayer)
  (bind _zaxis (Timeline|Movement Play)
    (:Update
      (Transformation|SetRelativeLocation (Variables|Default|GetHitBox) (Math|Vector|MakeVector 0.0 0.0 _zaxis) false false))))

(event EventDamager
  ;[1 0 1 1 100] HitByAoe
  (CallFunction|HitTarget))

(fn ConstructionScript)