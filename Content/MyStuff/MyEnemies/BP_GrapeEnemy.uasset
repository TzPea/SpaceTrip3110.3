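; BP_GrapeEnemy is a grape enemy that chases the player and bursts on contact, calling GotShot on them.
; AIMoveTo re-runs a second after each result while a timeline animates the mesh's height.
; Hits step down health, swapping meshes and materials, with a random ammo drop at zero.
; Grenades, area damage and lost health lead to death: Niagara effect, collision off, delayed destroy.
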(event OnComponentBeginOverlap(HitBox)
  (params (OverlappedComponent :type Primitive%20Component%20Object%20Reference) (OtherActor :type Actor%20Object%20Reference) (OtherComp :type Primitive%20Component%20Object%20Reference) (OtherBodyIndex :type Integer) (bFromSweep :type Boolean) (SweepResult :type Hit%20Result%20Structure%20%28by%20ref%29))
  ;[1 0 1 1 100] KillPlayer
  (bind _asbp_first_person_character (Utilities|Casting|CastToBP_FirstPersonCharacter OtherActor))
  (Audio|PlaySoundatLocation "/Game/Sounds/ShotgunSplat.ShotgunSplat" "0, 0, 0" "0, 0, 0" 1.0 1.0 0.0 0 0 0 0)
  (Default|GotShot _asbp_first_person_character)
  (CallFunction|Explode))

(event OnComponentHit(HitBox)
  (params (HitComponent :type Primitive%20Component%20Object%20Reference) (OtherActor :type Actor%20Object%20Reference) (OtherComp :type Primitive%20Component%20Object%20Reference) (NormalImpulse :type Vector :default "0, 0, 0") (Hit :type Hit%20Result%20Structure%20%28by%20ref%29))
  ;[1 0 1 1 100] Grenade Hit Death
  (bind _asbp_melon_grenade (Utilities|Casting|CastToBP_MelonGrenade OtherActor))
  (Default|Explode _asbp_melon_grenade)
  (CallFunction|Death))

(event Custom|Death
  ;[1 0 1 1 100] Death Logic
  (Components|Activation|Activate (Variables|Default|GetNiagara) false)
  (Collision|SetCollisionEnabled (Variables|Collision|GetCapsuleComponent) "NoCollision")
  (Utilities|FlowControl|Delay 3.0)
  (Actor|DestroyActor))

(event Custom|GoToPlayer
  ;[1 0 1 1 100] Chase Player
  (Variables|/Script/Engine.CharacterMovementComponent|SetMaxWalkSpeed (Variables|Character|GetCharacterMovement) (Variables|Default|GetMax%20Walk%20Speed))
  (AI|AIMoveTo self "0, 0, 0" (Game|GetPlayerCharacter 0) 0.0 false
    (:OnSuccess
      _)
    (:OnFail
      _))
  (Utilities|FlowControl|Delay 1.0)
  (CallFunction|GotoPlayer))

(event Custom|SpawnAmmo
  ;[1 0 1 1 100] SpawnAmmo
  (switch int (Math|Random|RandomIntegerinRange 1 (Variables|Default|GetAmmoChance))
    (:1
      (Game|SpawnActorfromClass (Variables|Default|GetAmmoTypes) (Math|Transform|MakeTransform (Transformation|GetWorldLocation (Variables|Collision|GetCapsuleComponent)) "0, 0, 0" "1.000000,1.000000,1.000000") "AdjustIfPossibleButDontSpawnIfColliding" "OverrideRootScale" 0 0))))

(event Custom|HitTarget
  (bind _charactermesh (Variables|Default|GetCharacterMesh))
  ;[1 0 1 1 100] Getting Hit
  (bind _result (Math|Integer|DecrementInt (Variables|Default|GetHealth))
    (:%20%20
      (bind _output_get (Variables|Default|SetHealth _result))
      (switch int _output_get
        (:0
          (CallFunction|SpawnAmmo)
          (Components|StaticMesh|SetStaticMesh _charactermesh 0)
          (CallFunction|Death))
        (:1
          (Components|StaticMesh|SetStaticMesh _charactermesh (Variables|Default|Gethealth1Mesh))
          (Rendering|Material|SetMaterial _charactermesh 0 "/Game/MyStuff/MyMaterials/MAT_GrapeLowHealth.MAT_GrapeLowHealth"))
        (:2
          (Components|StaticMesh|SetStaticMesh _charactermesh (Variables|Default|Gethealth2Mesh))
          (Rendering|Material|SetMaterial _charactermesh 0 "/Game/MyStuff/MyMaterials/MAT_GrapeMidHealth.MAT_GrapeMidHealth"))))))

(event Custom|Explode
  ;[1 0 1 1 100] Getting Hit
  (Components|StaticMesh|SetStaticMesh (Variables|Default|GetCharacterMesh) 0)
  (CallFunction|Death))

(event EventBeginPlay
  ;[1 0 1 1 100] Movement
  (bind _asbp_first_person_character (Utilities|Casting|CastToBP_FirstPersonCharacter (Game|GetPlayerCharacter 0)))
  (Variables|Default|SetPlayer _asbp_first_person_character)
  (CallFunction|GotoPlayer)
  (bind _zaxis (Timeline|Movement Play)
    (:Update
      (Transformation|SetRelativeLocation (Variables|Default|GetCharacterMesh) (Math|Vector|MakeVector 0.0 0.0 _zaxis) false false))))

(event EventDamager
  ;[1 0 1 1 100] HitByAoe
  (CallFunction|Explode))

(fn ConstructionScript)