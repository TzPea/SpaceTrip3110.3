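; BP_StrawberryEnemy is an enemy that chases the player via a repeating AI MoveTo while a timeline animates its mesh's height.
; HitTarget decrements health, swapping mesh and material at damage thresholds and dying at zero; AoE damage or a melon grenade hit kills it outright.
; Overlapping the player calls GotShot on them and kills the enemy.
; Death activates Niagara, randomly drops shotgun ammo, decrements the player's enemy count and destroys the actor.
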(event OnComponentHit(Sphere)
  (params (HitComponent :type Primitive%20Component%20Object%20Reference) (OtherActor :type Actor%20Object%20Reference) (OtherComp :type Primitive%20Component%20Object%20Reference) (NormalImpulse :type Vector :default "0, 0, 0") (Hit :type Hit%20Result%20Structure%20%28by%20ref%29))
  ;[1 0 1 1 100] Grenade Hit Death
  (bind _asbp_melon_grenade (Utilities|Casting|CastToBP_MelonGrenade OtherActor))
  (Default|Explode _asbp_melon_grenade)
  (CallFunction|Death))

(event OnComponentBeginOverlap(Sphere)
  (params (OverlappedComponent :type Primitive%20Component%20Object%20Reference) (OtherActor :type Actor%20Object%20Reference) (OtherComp :type Primitive%20Component%20Object%20Reference) (OtherBodyIndex :type Integer) (bFromSweep :type Boolean) (SweepResult :type Hit%20Result%20Structure%20%28by%20ref%29))
  ;[1 0 1 1 100] Kill Player
  (bind _asbp_first_person_character (Utilities|Casting|CastToBP_FirstPersonCharacter OtherActor))
  (Utilities|FlowControl|DoOnce false
    (:Completed
      (Audio|PlaySoundatLocation "/Game/Sounds/ShotgunSplat.ShotgunSplat" "0, 0, 0" "0, 0, 0" 1.0 1.0 0.0 0 0 0 0)
      (Default|GotShot _asbp_first_person_character)
      (CallFunction|Death))))

(event Custom|GoToPlayer
  ;[1 0 1 1 100] GoToPlayerLogic
  (Variables|/Script/Engine.CharacterMovementComponent|SetMaxWalkSpeed (Variables|Character|GetCharacterMovement) (Variables|Default|GetMax%20Walk%20Speed))
  (AI|AIMoveTo self "0, 0, 0" (Game|GetPlayerCharacter 0) 1.0 false
    (:OnSuccess
      _)
    (:OnFail
      _))
  (Utilities|FlowControl|Delay 1.0)
  (CallFunction|GotoPlayer))

(event Custom|Death
  (Components|Activation|Activate (Variables|Default|GetNiagara) false)
  (Rendering|SetVisibility (Variables|Default|GetSphere) false false)
  (Collision|SetCollisionEnabled (Variables|Collision|GetCapsuleComponent) "NoCollision")
  (Utilities|FlowControl|Delay 0.99)
  (Utilities|FlowControl|MultiGate true true -1
    (:Out%200
      (Game|SpawnActorfromClass "/Game/MyStuff/MyBlueprints/BP_ShotgunAmmoPickUp.BP_ShotgunAmmoPickUp_C" (Math|Transform|MakeTransform (Transformation|GetWorldLocation (Variables|Collision|GetCapsuleComponent)) "0, 0, 0" "1.000000,1.000000,1.000000") "Undefined" "OverrideRootScale" 0 0))
    (:Out%201
      _))
  (Utilities|FlowControl|Delay 0.1)
  (Default|DecrementEnemies (Variables|Default|GetPlayer))
  (Actor|DestroyActor))

(event Custom|HitTarget
  (bind _sphere (Variables|Default|GetSphere))
  ;[1 0 1 1 100] Getting Hit
  (bind _result (Math|Integer|DecrementInt (Variables|Default|GetHealth))
    (:%20%20
      (bind _output_get (Variables|Default|SetHealth _result))
      (switch int _output_get
        (:0
          (Components|StaticMesh|SetStaticMesh _sphere "/Game/MyStuff/MyMeshes/dead_strawb.dead_strawb")
          (Rendering|Material|SetMaterial _sphere 0 "/Game/MyStuff/MyMaterials/MAT_DeadStrawberry.MAT_DeadStrawberry")
          (CallFunction|Death))
        (:2
          (Components|StaticMesh|SetStaticMesh _sphere "/Game/MyStuff/MyMeshes/lowhealthstrawb.lowhealthstrawb")
          (Rendering|Material|SetMaterial _sphere 0 "/Game/MyStuff/MyMaterials/MAT_StrawberryLow.MAT_StrawberryLow"))
        (:4
          (Components|StaticMesh|SetStaticMesh _sphere "/Game/MyStuff/MyMeshes/strawbmidhealth.strawbmidhealth")
          (Rendering|Material|SetMaterial _sphere 0 "/Game/MyStuff/MyMaterials/MAT_StrawberryMid.MAT_StrawberryMid"))))))

(event EventBeginPlay
  (bind _asbp_first_person_character (Utilities|Casting|CastToBP_FirstPersonCharacter (Game|GetPlayerCharacter 0)))
  (Variables|Default|SetPlayer _asbp_first_person_character)
  (CallFunction|GotoPlayer)
  (bind _zaxis (Timeline|Timeline Play)
    (:Update
      (Transformation|SetRelativeLocation (Variables|Default|GetSphere) (Math|Vector|MakeVector 0.0 0.0 _zaxis) false false))))

(event EventDamager
  ;[1 0 1 1 100] HitByAoe
  (CallFunction|Death))

(fn ConstructionScript)