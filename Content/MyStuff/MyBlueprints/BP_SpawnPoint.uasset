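; Spawn point actor that periodically spawns one fruit enemy type (Grapes, Strawberry or Watermelon) at its Spawn component, chosen by EnemyTypes.
; After a start delay, SpawnAgain asks the first-person player character whether spawning is allowed.
; An allowed call sets a looping timer back onto SpawnAgain and spawns the AI pawn, so no timer starts if the first check fails.
; DecrementCounter lowers NumEnemies, which spawning here never reads.
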(event Custom|SpawnAgain
  (bind _spawn (Variables|Default|GetSpawn))
  (bind _returnvalue (Transformation|GetWorldTransform _spawn))
  (bind _spawn_2 (Default|CanSpawnEnemy (Variables|Default|GetPlayer)))
  (if _spawn_2
    (Utilities|Time|SetTimerbyEvent (delegate Custom|SpawnAgain) (Variables|Default|GetSpawnTimer) true)
    (switch Utilities|FlowControl|Switch|SwitchonEnum_EnemyTypes (Variables|Default|GetEnemyTypes)
      (:NewEnumerator1
        (AI|SpawnAIFromClass "/Game/MyStuff/MyEnemies/BP_GrapeEnemy.BP_GrapeEnemy_C" 0 (.location _returnvalue) "0, 0, 0" false 0))
      (:NewEnumerator0
        (AI|SpawnAIFromClass "/Game/MyStuff/MyEnemies/BP_StrawberryEnemy.BP_StrawberryEnemy_C" 0 (.location _returnvalue) "0, 0, 0" false 0))
      (:NewEnumerator2
        (AI|SpawnAIFromClass "/Game/MyStuff/MyEnemies/BP_WatermelonEnemy.BP_WatermelonEnemy_C" 0 (.location _returnvalue) "0, 0, 0" false 0)))))

(event Custom|DecrementCounter
  (Math|Integer|DecrementInt (Variables|Default|GetNumEnemies)))

(event EventBeginPlay
  (bind _asbp_first_person_character (Utilities|Casting|CastToBP_FirstPersonCharacter (Game|GetPlayerCharacter 0)))
  (Variables|Default|SetPlayer _asbp_first_person_character)
  (Utilities|FlowControl|Delay (Variables|Default|GetStartDelay))
  (CallFunction|SpawnAgain))

(fn ConstructionScript)