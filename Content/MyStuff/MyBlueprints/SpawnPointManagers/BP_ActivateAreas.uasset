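; BP_ActivateAreas unlocks an area once enough hardpoints have been completed.
; After a configurable start delay on BeginPlay, a self-calling Loop event polls the HardPointManager for its completed count every five seconds.
; When that count reaches HPNeededToActivate, it sets the AreaManager's unlocked flag and the polling stops.
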(event Custom|Loop
  (bind _returnvalue (Class|HardpointManager|GetHardpointsComplete (Variables|Default|GetHardPointManager)))
  (if (>= _returnvalue (Variables|Default|GetHPNeededToActivate))
    (Class|AreaManager|SetIsUnlocked (Variables|Default|GetAreaManager) true)
    (else
      (Utilities|FlowControl|Delay 5.0)
      (CallFunction|Loop))))

(event EventBeginPlay
  (Utilities|FlowControl|Delay (Variables|Default|GetLoopStartDelay))
  (CallFunction|Loop))

(fn ConstructionScript)