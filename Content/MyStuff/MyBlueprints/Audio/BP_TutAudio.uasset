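; BP_TutAudio is a trigger actor that plays a tutorial audio clip once when the first-person character enters its overlap component.
; A DoOnce gate keeps the audio from replaying on later overlaps.
; When AllowInput is off, it disables the character's input, waits for TimeToPlayAudio, then re-enables it.
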(event OnComponentBeginOverlap(Trigger)
  (params (OverlappedComponent :type Primitive%20Component%20Object%20Reference) (OtherActor :type Actor%20Object%20Reference) (OtherComp :type Primitive%20Component%20Object%20Reference) (OtherBodyIndex :type Integer) (bFromSweep :type Boolean) (SweepResult :type Hit%20Result%20Structure%20%28by%20ref%29))
  (bind _returnvalue (Game|GetPlayerController 0))
  (bind _asbp_first_person_character (Utilities|Casting|CastToBP_FirstPersonCharacter OtherActor))
  (Utilities|FlowControl|DoOnce false
    (:Completed
      (Audio|Components|Audio|Play (Variables|Default|GetAudio) 0.0)
      (if (not (Variables|Default|GetAllowInput))
        (Input|DisableInput _asbp_first_person_character _returnvalue)
        (Utilities|FlowControl|Delay (Variables|Default|GetTimeToPlayAudio))
        (Input|EnableInput _asbp_first_person_character _returnvalue)))))

(fn ConstructionScript)