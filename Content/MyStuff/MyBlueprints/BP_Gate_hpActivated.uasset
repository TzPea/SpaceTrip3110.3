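; A gate actor that opens once enough hardpoints have been completed.
; From BeginPlay it polls the hardpoint manager every five seconds until the completed count equals the required number.
; It then plays opening audio and a timeline that lerps the gate's relative location from closed to open, which stops the polling loop.
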(event Custom|HardpointCompetle
  (bind _returnvalue (Class|HardpointManager|GetHardpointsComplete (Variables|Default|GetHP_Manager)))
  (bind _output_get (Variables|Default|SetHPComplete _returnvalue))
  (if (== _output_get (Variables|Default|GetHardPointsNeededToOpen))
    (Audio|Components|Audio|Play (Variables|Default|GetGateOpenAudio) 0.0)
    (Variables|Default|SetGateOpen true)
    (bind _gate_open (Timeline|Gate_Open Play)
      (:Update
        (Transformation|SetRelativeLocation (Variables|Default|GetGate) (Math|Vector|Lerp(Vector) (Variables|Default|GetGate_Closed_Postion) (Variables|Default|GetGate_Open_Postion) _gate_open) false false)))))

(event Custom|Loop
  (Utilities|FlowControl|Delay 5.0)
  (if (not (Variables|Default|GetGateOpen))
    (CallFunction|HardpointCompetle)
    (CallFunction|Loop)))

(event EventBeginPlay
  (CallFunction|Loop)
  (bind _gate_open (Timeline|Gate_Open Reverse)
    (:Update
      (Transformation|SetRelativeLocation (Variables|Default|GetGate) (Math|Vector|Lerp(Vector) (Variables|Default|GetGate_Closed_Postion) (Variables|Default|GetGate_Open_Postion) _gate_open) false false))))

(fn ConstructionScript)