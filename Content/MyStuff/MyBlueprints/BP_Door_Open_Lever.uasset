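; Lever-operated gate that the first-person character can open once.
; A Box overlap sets InTrigger, which lets GeneralInteract hide the lever and, guarded by GateUsed, play the Gate_Open timeline.
; The timeline lerps the gate's relative location from closed to open position.
; BeginPlay runs the same timeline in reverse from its end, so the gate moves from open to closed at start.
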(event OnComponentBeginOverlap(Box)
  (params (OverlappedComponent :type Primitive%20Component%20Object%20Reference) (OtherActor :type Actor%20Object%20Reference) (OtherComp :type Primitive%20Component%20Object%20Reference) (OtherBodyIndex :type Integer) (bFromSweep :type Boolean) (SweepResult :type Hit%20Result%20Structure%20%28by%20ref%29))
  (Utilities|Casting|CastToBP_FirstPersonCharacter OtherActor)
  (Variables|Default|SetInTrigger true))

(event OnComponentEndOverlap(Box)
  (params (OverlappedComponent :type Primitive%20Component%20Object%20Reference) (OtherActor :type Actor%20Object%20Reference) (OtherComp :type Primitive%20Component%20Object%20Reference) (OtherBodyIndex :type Integer))
  (Utilities|Casting|CastToBP_FirstPersonCharacter OtherActor)
  (Variables|Default|SetInTrigger false))

(event EventGeneralInteract
  (params (Dmg :type Float%20%28double-precision%29))
  (if (Variables|Default|GetInTrigger)
    (Rendering|SetVisibility (Variables|Default|GetLever) false false)
    (if (not (Variables|Default|GetGate_Used))
      (Variables|Default|SetGate_Used true)
      (bind _gate_open (Timeline|Gate_Open Play)
        (:Update
          (Transformation|SetRelativeLocation (Variables|Default|GetGate) (Math|Vector|Lerp(Vector) (Variables|Default|GetGate_Closed_Postion) (Variables|Default|GetGate_Open_Postion) _gate_open) false false))))))

(event EventBeginPlay
  (bind _gate_open (Timeline|Gate_Open ReverseFromEnd)
    (:Update
      (Transformation|SetRelativeLocation (Variables|Default|GetGate) (Math|Vector|Lerp(Vector) (Variables|Default|GetGate_Closed_Postion) (Variables|Default|GetGate_Open_Postion) _gate_open) false false))))

(fn ConstructionScript)