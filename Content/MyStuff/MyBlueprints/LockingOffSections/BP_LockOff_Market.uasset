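; BP_LockOff_Market is a blocker actor that seals off the market section until hardpoint progress unlocks it.
; From BeginPlay it runs a self-calling loop that checks the HPManager's completed hardpoint count every five seconds.
; When that count equals exactly one, the actor destroys itself.
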(event Custom|MarketLO
  (bind _returnvalue (Class|HardpointManager|GetHardpointsComplete (Variables|Default|GetHP_Manager)))
  (bind _output_get (Variables|Default|Setint _returnvalue))
  (if (== _output_get 1)
    (Actor|DestroyActor)))

(event Custom|Loop
  (Utilities|FlowControl|Delay 5.0)
  (CallFunction|MarketLO)
  (CallFunction|Loop))

(event EventBeginPlay
  (CallFunction|Loop))

(fn ConstructionScript)