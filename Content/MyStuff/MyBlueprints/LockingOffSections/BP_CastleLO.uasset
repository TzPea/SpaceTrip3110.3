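; BP_CastleLO is a lock-off actor that blocks the castle section until enough hardpoints are completed.
; From BeginPlay it runs a self-calling loop that polls HPManager every five seconds for the completed hardpoint count.
; When the count equals five, it sets the AreaManager to unlocked and destroys itself.
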(event Custom|MarketLO2
  (bind _returnvalue (Class|HardpointManager|GetHardpointsComplete (Variables|Default|GetHP_Manager)))
  (bind _output_get (Variables|Default|SetHPComplete _returnvalue))
  (if (== _output_get 5)
    (Class|AreaManager|SetIsUnlocked (Variables|Default|GetAreaManager) true)
    (Actor|DestroyActor)))

(event Custom|Loop
  (Utilities|FlowControl|Delay 5.0)
  (CallFunction|MarketLO2)
  (CallFunction|Loop))

(event EventBeginPlay
  (CallFunction|Loop))

(fn ConstructionScript)