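; BP_LockOffSections is an actor that locks off a section until a required number of hardpoints is complete, then destroys itself.
; From BeginPlay, a self-calling Loop event uses a five-second Delay to poll HPManager for the completed hardpoint count.
; The actor is destroyed only when that count exactly equals its required amount.
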(event Custom|CheckHardpointCompleteAmount
  (bind _returnvalue (Class|HardpointManager|GetHardpointsComplete (Variables|Default|GetHP_Manager)))
  (bind _output_get (Variables|Default|SetHPComplete _returnvalue))
  (if (== _output_get (Variables|Default|GetHardPointsNeededToBeCompelete))
    (Actor|DestroyActor)))

(event Custom|Loop
  (Utilities|FlowControl|Delay 5.0)
  (CallFunction|CheckHardpointCompleteAmount)
  (CallFunction|Loop))

(event EventBeginPlay
  (CallFunction|Loop))

(fn ConstructionScript)