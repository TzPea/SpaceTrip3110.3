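; Enemy melon grenade actor that arcs toward a target and explodes on a timer.
; Launch solves a toss velocity for ProjectileMovement, while Tick orients the trail against travel and disables it when stopped or dead.
; BeginPlay swaps to a warning material before Explode plays effects and sphere-traces at the collision component's relative location.
; Hits implementing I_RecieveDamage receive damage messages; only that branch leads to delayed self-destruction.
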(event Custom|Explode
  (bind _collisioncomponent (Variables|MyProjectile|GetCollisionComponent))
  (bind _relativelocation (Variables|/Script/Engine.SceneComponent|GetRelativeLocation _collisioncomponent))
  ;[1 0 1 1 100] Explode Logic
  (Variables|Default|SetDead true)
  (Audio|PlaySoundatLocation "/Game/StarterContent/Audio/Explosion02.Explosion02" (Transformation|GetWorldLocation (Variables|MyProjectile|GetMelonade)) "0, 0, 0" 0.5 1.0 0.0 0 0 0 0)
  (Rendering|SetVisibility (Variables|MyProjectile|GetMelonade) false false)
  (Components|Activation|Activate (Variables|Default|GetNiagara) false)
  (bind _outhits (Collision|MultiSphereTraceByChannel _relativelocation _relativelocation 4e+02 "TraceTypeQuery1" false 0 "None"))
  (for _array_element _outhits
    (if (Utilities|DoesObjectImplementInterface (.HitActor (Collision|BreakHitResult _array_element)) "/Game/MyStuff/MyBlueprints/I_RecieveDamage.I_RecieveDamage_C")
      (Class|IRecieveDamage|DamageSend(Message) (.HitActor (Collision|BreakHitResult _array_element)))
      (Rendering|SetVisibility (Variables|MyProjectile|GetMelonade) false false)
      (Utilities|FlowControl|Delay 1.0)
      (Actor|DestroyActor))))

(event Custom|Launch
  (params (Origin :type Vector) (Target :type Vector))
  (bind _projectilemovement (Variables|Default|GetProjectileMovement))
  (bind (_tossvelocity _returnvalue) (Class|GameplayStatics|BlueprintSuggestProjectileVelocity Origin Target 1e+03 0.0 "DoNotTrace" 0.0 false false))
  (if _returnvalue
    (Variables|/Script/Engine.MovementComponent|SetVelocity _projectilemovement _tossvelocity)
    (else
      (Development|PrintString "Cant Reach")))
  (Components|Activation|Activate _projectilemovement false))

(event EventBeginPlay
  ;[1 0 1 1 100] Timer
  (Utilities|FlowControl|Delay 3.0)
  (Rendering|Material|SetMaterial (Variables|MyProjectile|GetMelonade) 0 "/Game/MyStuff/MyMaterials/MAT_MelonadeExplode.MAT_MelonadeExplode")
  (Utilities|FlowControl|Delay 1.0)
  (CallFunction|Explode))

(event EventTick
  (params (DeltaSeconds :type Float%20%28single-precision%29))
  (bind _trail (Variables|Default|GetTrail))
  (bind _projectilemovement (Variables|Default|GetProjectileMovement))
  (bind _velocity (Variables|/Script/Engine.MovementComponent|GetVelocity _projectilemovement))
  (if (Utilities|Operators|EqualEqual :A _velocity :ErrorTolerance 0.1)
    (Components|Activation|SetActive _trail false false :!label _label)
    (elif (Variables|Default|GetDead)
      (goto _label)
      (else
        (Components|Activation|SetActive _trail true false))))
  (Transformation|SetRelativeRotation _trail (Math|Conversions|RotationFromXVector (Math|Vector|NegateVector (Math|Vector|Normalize _velocity))) false false))

(fn ConstructionScript)

(fn Damager
  (return))