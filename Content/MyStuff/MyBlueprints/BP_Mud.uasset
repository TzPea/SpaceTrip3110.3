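; BP_Mud is a mud hazard that slows the player and enemies while they overlap its Trigger.
; Entering plays MudSplat for the player, lowers walk speed and lengthens the dash cooldown; leaving sets both to fixed values.
; Enemies derived from EnemyBase lose a flat amount of walk speed and get it back from EnemyWalkSpeed, a single variable overwritten by each entering enemy.
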(event OnComponentBeginOverlap(Trigger)
  (params (OverlappedComponent :type Primitive%20Component%20Object%20Reference) (OtherActor :type Actor%20Object%20Reference) (OtherComp :type Primitive%20Component%20Object%20Reference) (OtherBodyIndex :type Integer) (bFromSweep :type Boolean) (SweepResult :type Hit%20Result%20Structure%20%28by%20ref%29))
  (Utilities|FlowControl|Sequence
    (:then_0
      (bind _asbp_first_person_character (Utilities|Casting|CastToBP_FirstPersonCharacter OtherActor))
      (Audio|Components|Audio|Play (Variables|Default|GetMud_Splat) 0.0)
      (Variables|/Script/Engine.CharacterMovementComponent|SetMaxWalkSpeed (Variables|/Script/Engine.Character|GetCharacterMovement _asbp_first_person_character) 3e+02)
      (Variables|/Game/FPS_Stuff/FirstPerson/Blueprints/BP_FirstPersonCharacter.BP_FirstPersonCharacter_C|SetDash%20CoolDown _asbp_first_person_character 3.0))
    (:then_1
      (bind _asenemy_base (Utilities|Casting|CastToEnemyBase OtherActor))
      (Variables|Default|SetEnemy%20Walk%20Speed (Variables|/Script/Engine.CharacterMovementComponent|GetMaxWalkSpeed (Variables|/Script/Engine.Character|GetCharacterMovement _asenemy_base)))
      (Variables|/Script/Engine.CharacterMovementComponent|SetMaxWalkSpeed (Variables|/Script/Engine.Character|GetCharacterMovement _asenemy_base) (- (Variables|/Script/Engine.CharacterMovementComponent|GetMaxWalkSpeed (Variables|/Script/Engine.Character|GetCharacterMovement _asenemy_base)) 1e+02)))))

(event OnComponentEndOverlap(Trigger)
  (params (OverlappedComponent :type Primitive%20Component%20Object%20Reference) (OtherActor :type Actor%20Object%20Reference) (OtherComp :type Primitive%20Component%20Object%20Reference) (OtherBodyIndex :type Integer))
  (Utilities|FlowControl|Sequence
    (:then_0
      (bind _asbp_first_person_character (Utilities|Casting|CastToBP_FirstPersonCharacter OtherActor))
      (Variables|/Script/Engine.CharacterMovementComponent|SetMaxWalkSpeed (Variables|/Script/Engine.Character|GetCharacterMovement _asbp_first_person_character) 5e+02)
      (Variables|/Game/FPS_Stuff/FirstPerson/Blueprints/BP_FirstPersonCharacter.BP_FirstPersonCharacter_C|SetDash%20CoolDown _asbp_first_person_character 1.0))
    (:then_1
      (bind _asenemy_base (Utilities|Casting|CastToEnemyBase OtherActor))
      (Variables|/Script/Engine.CharacterMovementComponent|SetMaxWalkSpeed (Variables|/Script/Engine.Character|GetCharacterMovement _asenemy_base) (Variables|Default|GetEnemy%20Walk%20Speed)))))

(fn ConstructionScript)