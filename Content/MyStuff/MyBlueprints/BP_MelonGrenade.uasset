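; BP_MelonGrenade is a timed melon grenade projectile that switches to a warning material after three seconds and explodes one second later.
; Tick aims the trail opposite the velocity and disables it when stopped or dead.
; Explode plays sound and effects, then sphere-traces to message hit actors implementing I_Damager.
; The delayed self-destruct runs inside the hit loop, so it depends on the trace hitting something.
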(event Custom|Explode
  (bind _collisioncomponent (Variables|MyProjectile|GetCollisionComponent))
  (bind _relativelocation (Variables|/Script/Engine.SceneComponent|GetRelativeLocation _collisioncomponent))
  (Variables|Default|SetDead true)
  (Audio|PlaySoundatLocation "/Game/StarterContent/Audio/Explosion02.Explosion02" (Transformation|GetWorldLocation (Variables|MyProjectile|GetMelonade)) "0, 0, 0" 0.5 1.0 0.0 0 0 0 0)
  (Rendering|SetVisibility (Variables|MyProjectile|GetMelonade) false false)
  (Components|Activation|Activate (Variables|Default|GetNiagara) false)
  (bind _outhits (Collision|MultiSphereTraceByChannel _relativelocation _relativelocation 5e+02 "TraceTypeQuery1" false 0 "None"))
  (for _array_element _outhits
    (if (Utilities|DoesObjectImplementInterface (.HitActor (Collision|BreakHitResult _array_element)) "/Game/MyStuff/MyBlueprints/I_Damager.I_Damager_C")
      (Class|IDamager|Damager(Message) (.HitActor (Collision|BreakHitResult _array_element))))
    (Rendering|SetVisibility (Variables|MyProjectile|GetMelonade) false false)
    (Components|Activation|SetActive (Variables|Default|GetExplosion) true false)
    (Utilities|FlowControl|Delay 1.0)
    (Actor|DestroyActor)))

(event EventBeginPlay
  (Utilities|FlowControl|Delay 3.0)
  (Rendering|Material|SetMaterial (Variables|MyProjectile|GetMelonade) 0 "/Game/MyStuff/MyMaterials/MAT_MelonadeExplode.MAT_MelonadeExplode")
  (Utilities|FlowControl|Delay 1.0)
  (CallFunction|Explode))

(event EventTick
  (params (DeltaSeconds :type Float%20%28single-precision%29))
  (bind _trail (Variables|Default|GetTrail))
  (bind _projectilemovement (Variables|Default|GetProjectileMovement))
  (bind _velocity (Variables|/Script/Engine.MovementComponent|GetVelocity _projectilemovement))
  (if (Utilities|Operators|EqualEqual :A _velocity :ErrorTolerance 0.1)
    (Components|Activation|SetActive _trail false false :!label _label)
    (elif (Variables|Default|GetDead)
      (goto _label)
      (else
        (Components|Activation|SetActive _trail true false))))
  (Transformation|SetRelativeRotation _trail (Math|Conversions|RotationFromXVector (Math|Vector|NegateVector (Math|Vector|Normalize _velocity))) false false))

(fn ConstructionScript)

(fn Damager
  (return))