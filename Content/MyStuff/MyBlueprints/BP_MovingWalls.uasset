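; BP_MovingWalls is a wall actor that moves between two relative positions, starting at BeginPlay.
; The Movement_Up timeline lerps the Wall component from UpPos to DownPos.
; Each timeline update also feeds a random-length Delay between DelayTimeMin and DelayTimeMax, which calls the start event again.
; A separate custom event reverses the timeline from its end, with no caller in this graph.
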(event Custom|MovingWall_Start
  (bind _newtrack_1 (Timeline|Movement_Up PlayFromStart)
    (:Update
      (Transformation|SetRelativeLocation (Variables|Default|GetWall) (Math|Vector|Lerp(Vector) (Variables|Default|GetUp_Pos) (Variables|Default|GetDown_Pos) _newtrack_1) false false)
      (Utilities|FlowControl|Delay (Math|Random|RandomFloatinRange (Variables|Default|GetDelayTime_Min) (Variables|Default|GetDelayTime_Max)))
      (CallFunction|MovingWallStart))))

(event Custom|CustomEvent
  (bind _newtrack_1 (Timeline|Movement_Up ReverseFromEnd)
    (:Update
      (Transformation|SetRelativeLocation (Variables|Default|GetWall) (Math|Vector|Lerp(Vector) (Variables|Default|GetUp_Pos) (Variables|Default|GetDown_Pos) _newtrack_1) false false)
      (Utilities|FlowControl|Delay (Math|Random|RandomFloatinRange (Variables|Default|GetDelayTime_Min) (Variables|Default|GetDelayTime_Max)))
      (CallFunction|MovingWallStart))))

(event EventBeginPlay
  (CallFunction|MovingWallStart))

(fn ConstructionScript)