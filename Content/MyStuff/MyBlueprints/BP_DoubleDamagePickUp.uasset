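; BP_DoubleDamagePickUp is a bottle pickup that activates double damage on the first-person character that overlaps its box.
; On BeginPlay a Float timeline moves the bottle vertically, and its update drives a Rotate timeline that spins the bottle's yaw.
; The rotation update also starts a DeleteTime delay that destroys the pickup if uncollected.
; Collection plays a gulp and destroys the actor after a short delay.
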(event OnComponentBeginOverlap(Box)
  (params (OverlappedComponent :type Primitive%20Component%20Object%20Reference) (OtherActor :type Actor%20Object%20Reference) (OtherComp :type Primitive%20Component%20Object%20Reference) (OtherBodyIndex :type Integer) (bFromSweep :type Boolean) (SweepResult :type Hit%20Result%20Structure%20%28by%20ref%29))
  (bind _asbp_first_person_character (Utilities|Casting|CastToBP_FirstPersonCharacter OtherActor))
  (Default|ActivateDoubleDamage _asbp_first_person_character)
  (Audio|Components|Audio|Play (Variables|Default|GetGulp) 0.0)
  (Utilities|FlowControl|Delay 0.5)
  (Actor|DestroyActor))

(event EventBeginPlay
  (bind _bottle (Variables|Default|GetBottle))
  (bind _newtrack_0 (Timeline|Float Play)
    (:Update
      (Transformation|SetRelativeLocation _bottle (Math|Vector|MakeVector 0.0 0.0 _newtrack_0) false false)
      (bind _zrotate (Timeline|Rotate Play)
        (:Update
          (Transformation|SetRelativeRotation _bottle (Math|Rotator|MakeRotator 0.0 0.0 _zrotate) false false)
          (Utilities|FlowControl|Delay (Variables|Default|GetDelete%20Time))
          (Actor|DestroyActor))))))

(fn ConstructionScript)