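; BP_Tp_TG is a two-portal teleporter that unlocks once the player has completed at least six hardpoints.
; Overlapping the activation trigger queries the HardPointManager and, when the count is met, swaps both portal materials and sets Active.
; While active, each of the two portal triggers teleports the overlapping first-person character to its own stored location and rotation.
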(event OnComponentBeginOverlap(Trigger1)
  (params (OverlappedComponent :type Primitive%20Component%20Object%20Reference) (OtherActor :type Actor%20Object%20Reference) (OtherComp :type Primitive%20Component%20Object%20Reference) (OtherBodyIndex :type Integer) (bFromSweep :type Boolean) (SweepResult :type Hit%20Result%20Structure%20%28by%20ref%29))
  ;[1 1 1] TP_1
  (bind _asbp_first_person_character (Utilities|Casting|CastToBP_FirstPersonCharacter OtherActor))
  (if (Variables|Default|GetActive)
    (Transformation|Teleport _asbp_first_person_character (Variables|Default|GetTP1_Location) (Variables|Default|GetTP1_Rotation))))

(event OnComponentBeginOverlap(Trigger_ToActivate)
  (params (OverlappedComponent :type Primitive%20Component%20Object%20Reference) (OtherActor :type Actor%20Object%20Reference) (OtherComp :type Primitive%20Component%20Object%20Reference) (OtherBodyIndex :type Integer) (bFromSweep :type Boolean) (SweepResult :type Hit%20Result%20Structure%20%28by%20ref%29))
  (Utilities|Casting|CastToBP_FirstPersonCharacter OtherActor)
  (bind _returnvalue (Class|HardpointManager|GetHardpointsComplete (Variables|Default|GetHardPoint_Manager)))
  (if (>= _returnvalue 6)
    (Rendering|Material|SetMaterial (Variables|Default|GetPortal2) 0 "/Game/MyStuff/MyMaterials/MAT_MelonChunk.MAT_MelonChunk")
    (Variables|Default|SetActive true)))

(event OnComponentBeginOverlap(Trigger2)
  (params (OverlappedComponent :type Primitive%20Component%20Object%20Reference) (OtherActor :type Actor%20Object%20Reference) (OtherComp :type Primitive%20Component%20Object%20Reference) (OtherBodyIndex :type Integer) (bFromSweep :type Boolean) (SweepResult :type Hit%20Result%20Structure%20%28by%20ref%29))
  ;[1 1 1] TP_2
  (bind _asbp_first_person_character (Utilities|Casting|CastToBP_FirstPersonCharacter OtherActor))
  (if (Variables|Default|GetActive)
    (Transformation|Teleport _asbp_first_person_character (Variables|Default|GetTP2_Location) (Variables|Default|GetTP2_Rotation))))

(fn ConstructionScript)