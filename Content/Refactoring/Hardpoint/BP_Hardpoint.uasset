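; Hardpoint Blueprint for a seed the player starts by interacting while it is awake, growing a mushroom toward a timer goal.
; Tick fades ambient sound, swaps beacon effects for domes once started, and changes dome material by active state.
; It writes timer progress and name to the first-person character and scales the mushroom by that progress.
; Interaction plays a rate-limited growth sound, or flags the seed as not ready when asleep.
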(event EventGeneralInteract
  (params (Dmg :type Float%20%28double-precision%29))
  (bind _returnvalue (Class|Hardpoint|CheckIsAwake))
  (if _returnvalue
    (Class|Hardpoint|SetIsStarted true)
    (Utilities|FlowControl|DoOnce false :!label _label
      (:Completed
        (Audio|PlaySoundatLocation "/Game/Sounds/GrowingMushroom.GrowingMushroom" "0, 0, 0" "0, 0, 0" 1.0 1.0 0.0 0 0 0 0)
        (Utilities|FlowControl|Delay 6e+01)
        (goto _label Reset)))
    (else
      (Utilities|FlowControl|DoOnce false :!label _label_2
        (:Completed
          (Variables|/Game/FPS_Stuff/FirstPerson/Blueprints/BP_FirstPersonCharacter.BP_FirstPersonCharacter_C|SetSeedNotReady (Variables|Default|GetPlayer) true)
          (Utilities|FlowControl|Delay 3.0)
          (Variables|/Game/FPS_Stuff/FirstPerson/Blueprints/BP_FirstPersonCharacter.BP_FirstPersonCharacter_C|SetSeedNotReady (Variables|Default|GetPlayer) true)
          (goto _label_2 Reset))))))

(event EventTick
  (params (DeltaSeconds :type Float%20%28single-precision%29))
  (bind _dome (Variables|Default|GetDome))
  (bind _dome1 (Variables|Default|GetDome1))
  (bind _beam (Variables|Default|GetBeam))
  (bind _fantasysounds (Variables|Default|GetFantasySounds))
  (bind _returnvalue (Class|Hardpoint|CheckIsAwake))
  (if _returnvalue
    (if (Variables|Default|GetisStarted)
      (Audio|Components|Audio|AdjustVolume _fantasysounds 3.0 0.0 "Logarithmic" :!class /Script/Engine.AudioComponent)
      (Rendering|SetVisibility _beam false false)
      (Rendering|SetVisibility _dome true false)
      (bind _asbp_first_person_character (Utilities|Casting|CastToBP_FirstPersonCharacter (Game|GetPlayerCharacter 0)))
      (bind _returnvalue_2 (Class|Hardpoint|GetTimer))
      (bind _output_get (Variables|/Game/FPS_Stuff/FirstPerson/Blueprints/BP_FirstPersonCharacter.BP_FirstPersonCharacter_C|SetHardpointPercentage _asbp_first_person_character _returnvalue_2))
      (bind _returnvalue_3 (Class|Hardpoint|GetName))
      (Variables|/Game/FPS_Stuff/FirstPerson/Blueprints/BP_FirstPersonCharacter.BP_FirstPersonCharacter_C|SetCurrentHardpoint _asbp_first_person_character _returnvalue_3)
      (Transformation|SetWorldScale3D (Variables|Default|GetMushroomParent) (Math|Vector|Lerp(Vector) "0, 0, 0" "100.000000,100.000000,100.000000" (/ _output_get (Variables|Default|GetgoalTime))))
      (else
        (Audio|Components|Audio|AdjustVolume _fantasysounds 1.0 1.0 "Logarithmic" :!class /Script/Engine.AudioComponent)
        (Rendering|SetVisibility _beam true false)
        (Rendering|SetVisibility _dome false false :!label _label)))
    (else
      (goto _label)))
  (bind _returnvalue_4 (Class|Hardpoint|GetIsActive))
  (if _returnvalue_4
    (Rendering|Material|SetMaterial _dome1 0 "/Game/Mesh/M_GradientInsidePanner.M_GradientInsidePanner")
    (else
      (Rendering|Material|SetMaterial _dome1 0 "/Game/Mesh/M_GradientPanner.M_GradientPanner")))
  (bind _returnvalue_5 (Class|Hardpoint|GetTimer))
  (if (>= (Variables|Default|GetgoalTime) _returnvalue_5)
    (Utilities|FlowControl|Delay 3.0)
    (Transformation|SetWorldScale3D (Variables|Default|GetMushroomParent) "1.000000,1.000000,1.000000")))

(fn ConstructionScript)