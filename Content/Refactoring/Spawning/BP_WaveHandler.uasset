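; BP_WaveHandler watches the current wave number and relays wave changes to the first-person player character.
; On BeginPlay it caches the value from GetWave, then polls it every Tick, casting the player character each frame.
; On a change it updates the character's CurrentWave and runs ShowFont, which raises NewWaveStarted for a few seconds, clears it, then ends on a trailing delay.
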(event EventBeginPlay
  (Utilities|Casting|CastToBP_FirstPersonCharacter (Game|GetPlayerCharacter 0))
  (bind _returnvalue (Class|WaveHandler|GetWave))
  (Variables|Default|SetCachedWave _returnvalue))

(event EventTick
  (params (DeltaSeconds :type Float%20%28single-precision%29))
  (bind _asbp_first_person_character (Utilities|Casting|CastToBP_FirstPersonCharacter (Game|GetPlayerCharacter 0)))
  (bind _returnvalue (Class|WaveHandler|GetWave))
  (if (!= _returnvalue (Variables|Default|GetCachedWave))
    (bind _output_get (Variables|Default|SetCachedWave _returnvalue))
    (Variables|/Game/FPS_Stuff/FirstPerson/Blueprints/BP_FirstPersonCharacter.BP_FirstPersonCharacter_C|SetCurrentWave _asbp_first_person_character _output_get)
    (Utilities|ShowFont _asbp_first_person_character _asbp_first_person_character)))

(fn ConstructionScript)