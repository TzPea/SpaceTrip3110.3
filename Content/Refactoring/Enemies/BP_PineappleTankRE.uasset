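; Pineapple tank enemy that bobs with an animated scale and lobs BP_EnemyGrenade at the player.
; Tick fires it when the player is within 1000 units, with a DoOnce reset after a delay to pace shots.
; A direct BP_MelonGrenade hit detonates the grenade and calls HitActor five times.
; HitByGrenade, also triggered by a custom event, joins that chain partway for two hits.
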(event OnComponentHit(meshComp)
  (params (HitComponent :type Primitive%20Component%20Object%20Reference) (OtherActor :type Actor%20Object%20Reference) (OtherComp :type Primitive%20Component%20Object%20Reference) (NormalImpulse :type Vector :default "0, 0, 0") (Hit :type Hit%20Result%20Structure%20%28by%20ref%29))
  ;[1 0 1 1 100] Grenade Hit Death
  (bind _asbp_melon_grenade (Utilities|Casting|CastToBP_MelonGrenade OtherActor))
  (Default|Explode _asbp_melon_grenade)
  (Class|EnemyBase|HitActor)
  (Class|EnemyBase|HitActor)
  (Class|EnemyBase|HitActor)
  (Class|EnemyBase|HitActor)
  (Class|EnemyBase|HitActor))

(event Custom|TankFireReset
  (bind _returnvalue (Game|GetPlayerCharacter 0))
  (bind _spawngrenade (Variables|Default|GetSpawnGrenade))
  (bind _returnvalue_2 (Transformation|GetWorldLocation _spawngrenade))
  (bind _capsulecomponent (Variables|/Script/Engine.Character|GetCapsuleComponent _returnvalue))
  (bind _returnvalue_3 (Transformation|GetWorldLocation _capsulecomponent))
  ;[1 0 1 1 100] Firing Logic
  (Utilities|FlowControl|DoOnce false) ; enters at Reset
)

(event Custom|HitByGrenade
  ;[1 0 1 1 100] Grenade Hit Death
  (Class|EnemyBase|HitActor)
  (Class|EnemyBase|HitActor))

(event Custom|TankFire
  (bind _returnvalue (Game|GetPlayerCharacter 0))
  (bind _spawngrenade (Variables|Default|GetSpawnGrenade))
  (bind _returnvalue_2 (Transformation|GetWorldLocation _spawngrenade))
  (bind _capsulecomponent (Variables|/Script/Engine.Character|GetCapsuleComponent _returnvalue))
  (bind _returnvalue_3 (Transformation|GetWorldLocation _capsulecomponent))
  ;[1 0 1 1 100] Firing Logic
  (if (Variables|Default|GetCanFire)
    (Utilities|FlowControl|DoOnce false
      (:Completed
        (bind _returnvalue_4 (Game|SpawnActorfromClass "/Game/MyStuff/MyBlueprints/BP_EnemyGrenade.BP_EnemyGrenade_C" (Math|Transform|MakeTransform _returnvalue_2 (Math|Rotator|FindLookatRotation _returnvalue_2 _returnvalue_3) "1.000000,1.000000,1.000000") "Undefined" "MultiplyWithRoot" 0 "0.000000,0.000000,0.000000" 0))
        (Default|Launch _returnvalue_4 _returnvalue_2 _returnvalue_3)
        (Utilities|FlowControl|Delay 4.8)
        (Audio|Components|Audio|Play (Variables|Default|GetGrenadeFire) 0.0)
        (CallFunction|TankFireReset)))))

(event Custom|CustomEvent
  ;[1 0 1 1 100] HitByAoe
  (CallFunction|HitbyGrenade))

(event EventBeginPlay
  ;[1 0 1 1 100] Animations
  (bind _asbp_first_person_character (Utilities|Casting|CastToBP_FirstPersonCharacter (Game|GetPlayerCharacter 0)))
  (Variables|Default|SetPlayer _asbp_first_person_character)
  (bind _zaxis (Timeline|Bobbing Play)
    (:Update
      (Transformation|SetRelativeLocation (Variables|Default|GetmeshComp) (Math|Vector|MakeVector 0.0 0.0 _zaxis) false false)
      (bind (_direction _scale _width) (Timeline|TankScale Play)
        (:Update
          (Transformation|SetWorldScale3D (Variables|Default|GettankMeshComp) (Math|Vector|MakeVector _width _width _scale)))))))

(event EventTick
  (params (DeltaSeconds :type Float%20%28single-precision%29))
  ;[1 0 1 1 100] Distance Check
  (if (>= (Math|Vector|Distance(Vector) (Transformation|GetWorldLocation (Variables|Default|GetSpawnGrenade)) (Transformation|GetWorldLocation (Variables|/Script/Engine.Character|GetCapsuleComponent (Game|GetPlayerCharacter 0)))) 1e+03)
    (if (<= (Variables|/Game/FPS_Stuff/FirstPerson/Blueprints/BP_FirstPersonCharacter.BP_FirstPersonCharacter_C|GetHealthAmount (Variables|Default|GetPlayer)) 0.0)
      (Variables|Default|SetCanFire false))
    (else
      (Variables|Default|SetCanFire true)
      (CallFunction|TankFire))))

(fn ConstructionScript)