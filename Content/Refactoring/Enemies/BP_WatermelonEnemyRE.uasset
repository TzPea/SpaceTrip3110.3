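; BP_WatermelonEnemyRE is a watermelon enemy that damages the player on contact and dies in the process.
; HitBox overlap with the first-person character plays a splat sound and calls GotShot on the player, then OnDeath.
; A HitBox hit from a melon grenade detonates it and kills the enemy, as does a custom event for area-of-effect hits.
; Tick plays a Timeline that animates the mesh's relative Z.
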(event OnComponentBeginOverlap(HitBox)
  (params (OverlappedComponent :type Primitive%20Component%20Object%20Reference) (OtherActor :type Actor%20Object%20Reference) (OtherComp :type Primitive%20Component%20Object%20Reference) (OtherBodyIndex :type Integer) (bFromSweep :type Boolean) (SweepResult :type Hit%20Result%20Structure%20%28by%20ref%29))
  ;[1 0 1 1 100] KillPlayer
  (bind _asbp_first_person_character (Utilities|Casting|CastToBP_FirstPersonCharacter OtherActor))
  (Audio|PlaySoundatLocation "/Game/Sounds/ShotgunSplat.ShotgunSplat" "0, 0, 0" "0, 0, 0" 1.0 1.0 0.0 0 0 0 0)
  (Default|GotShot _asbp_first_person_character)
  (Class|EnemyBase|OnDeath))

(event OnComponentHit(HitBox)
  (params (HitComponent :type Primitive%20Component%20Object%20Reference) (OtherActor :type Actor%20Object%20Reference) (OtherComp :type Primitive%20Component%20Object%20Reference) (NormalImpulse :type Vector :default "0, 0, 0") (Hit :type Hit%20Result%20Structure%20%28by%20ref%29))
  ;[1 0 1 1 100] Grenade Hit Death
  (bind _asbp_melon_grenade (Utilities|Casting|CastToBP_MelonGrenade OtherActor))
  (Default|Explode _asbp_melon_grenade)
  (Class|EnemyBase|OnDeath))

(event Custom|CustomEvent
  ;[1 0 1 1 100] HitByAoe
  (Class|EnemyBase|OnDeath))

(event Collision|EventActorBeginOverlap
  (params (OtherActor :type Actor%20Object%20Reference)))

(event EventTick
  (params (DeltaSeconds :type Float%20%28single-precision%29))
  ;[1 0 1 1 100] Movement
  (bind _newtrack_0 (Timeline|Timeline Play)
    (:Update
      (Transformation|SetRelativeLocation (Variables|Default|GetmeshComp) (Math|Vector|MakeVector 0.0 0.0 _newtrack_0) false false))))

(fn ConstructionScript)